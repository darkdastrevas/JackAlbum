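; BP_Bern is a talkable character (Personagens folder) that shows dialogue and a quest notification.
; Each Talk call advances an index through DialogueFirst, or DialogueSecond when the player's TakeCaixa is set, displaying lines in WB_dialogue.
; DialogueFirst's length bounds both sets.
; At the end it removes the dialogue and, unless Quest4Ref is invalid and TakeCaixa is set, creates WBP_Quest4 with timed slide animations.
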(event `self.Talk`
  (bind _quest4ref (`self.quest4Ref`))
  ;[0 0 0] Diálogo
  (bind _asbp_third_person_character (cast `/Game/Blueprints/Personagens/BP_ThirdPersonCharacter` (`GameplayStatics.GetPlayerCharacter` 0)))
  (`/Engine/EditorBlueprintResources/StandardMacros.IncrementInt` (`self.talkindex`)
    (:`  `
      (if (< (`self.talkindex`) (`KismetArrayLibrary.Array_Length` (`self.dialogue_first`)))
        (bind _takecaixa (`/Game/Blueprints/Personagens/BP_ThirdPersonCharacter.takeCaixa` _asbp_third_person_character))
        (if _takecaixa
          (set `self.active_dialogue` (`self.dialogue_second`))
          (else
            (set `self.active_dialogue` (`self.dialogue_first`))))
        (`self.UI`
          (:`then`
            _)
          (:`else`
            (bind _returnvalue (`|CreateWidget` "/Game/Blueprints/Widgets/WB_dialogue.WB_dialogue_C" (`GameplayStatics.GetPlayerController` 0)))
            (bind _output_get (set `self.UI` _returnvalue))
            (`UserWidget.AddToViewport` _output_get 0)))
        (`TextBlock.SetText` (`/Game/Blueprints/Widgets/WB_dialogue.TalkText` (`self.UI`)) (`KismetTextLibrary.Conv_StringToText` (`|GetArrayItem` (`self.active_dialogue`) (`self.talkindex`))))
        (set `self.hasBeenInteracted` true)
        (else
          (`Widget.RemoveFromParent` (`self.UI`))
          (set `self.UI` null)
          (set `self.talkindex` -1)
          (if (not (and (not (`KismetSystemLibrary.IsValid` (`self.quest4Ref`))) _takecaixa))
            (bind _returnvalue_2 (`|CreateWidget` "/Game/Blueprints/Widgets/WBP_Quest4.WBP_Quest4_C"))
            (set `self.quest4Ref` _returnvalue_2)
            (`UserWidget.AddToViewport` _returnvalue_2 0)
            (`KismetSystemLibrary.Delay` 2.0)
            (`UserWidget.PlayAnimation` _returnvalue_2 (`/Game/Blueprints/Widgets/WBP_Quest4.SlideIn` _quest4ref) 0.0 1 "Forward" 1.0 false)
            (`KismetSystemLibrary.Delay` 5.0)
            (`UserWidget.PlayAnimation` _quest4ref (`/Game/Blueprints/Widgets/WBP_Quest4.SlideOut` _quest4ref) 0.0 1 "Forward" 1.0 false)
            (set `self.talkindex` -1)))))))

(fn `UserConstructionScript`)