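; Main player character Blueprint (Cin) handling movement, jumping, item carrying and the hat-selector toggle.
; Axis inputs drive world-space movement facing velocity, with delay-gated jumps and a brief movement lock on landing.
; E capsule-traces for physics bodies, attaching them hidden and non-colliding to GrabPoint, or releases them, with poof effects.
; Holding blocks the PC_SwitchHat selector, and an older PhysicsConstraint grab remains unconnected.
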(event `Key|E`
  (params (Key :type "Key Structure"))
  ;[1 1 1] salvo por preucaução
)

(event `InputAction|SwitchHatToggle`
  (params (Key :type "Key Structure"))
  ;[0 0 0] Trocar chapéu
  (:`Pressed`
    (if (not (`self.IsHolding`))
      (bind _aspc_switch_hat (cast `/Game/Blueprints/PC_SwitchHat` (`GameplayStatics.GetPlayerController` 0)))
      (`/Game/Blueprints/PC_SwitchHat.ShowWidgetSelector` _aspc_switch_hat)))
  (:`Released`
    (if (`KismetSystemLibrary.IsValid` _aspc_switch_hat)
      (`/Game/Blueprints/PC_SwitchHat.HideWidgetSelector` _aspc_switch_hat))))

(event `self.OnLanded`
  (params (Hit :type "HitResult Structure (by ref)"))
  ;[0.09031 0.2878 0.6719] Logica do pulo
  (set `self.canMove` false)
  (`KismetSystemLibrary.Delay` 0.4)
  (set `self.isLanded` true)
  (set `self.canMove` true))

(event `InputAxis|Go Forward/ Backwards`
  (params (AxisValue :type "Float (single-precision)"))
  (bind _returnvalue (`self.K2_GetActorLocation`))
  ;[0.02137 0.1173 0.3385] Movimento Básico
  (bind _output_get (set `self.AxisY` AxisValue))
  (if (`self.canMove`) :!label _label
    (bind _returnvalue_2 (`KismetMathLibrary.Normal` (`KismetMathLibrary.MakeVector` _output_get (stale `InputAxis|Go Right/ Left` _output_get))))
    (`self.AddMovementInput` _returnvalue_2)
    (if (and (not (`NavMovementComponent.IsFalling` (`self.CharacterMovement`))) (> (`KismetMathLibrary.VSize` _returnvalue_2) 0.1))
      (`self.K2_SetActorRotation` (`KismetMathLibrary.FindLookAtRotation` _returnvalue (+ _returnvalue (`self.GetVelocity`)))))))

(event `InputAction|Jump`
  (params (Key :type "Key Structure"))
  ;[0.09031 0.2878 0.6719] Logica do pulo
  (:`Pressed`
    (if (and (`self.isLanded`) (not (`self.IsJumping`)))
      (`self.Jump`)
      (set `self.IsJumping` true)
      (`KismetSystemLibrary.Delay` 0.75)
      (set `self.IsJumping` false))))

(event `InputAxis|Go Right/ Left`
  (params (AxisValue :type "Float (single-precision)"))
  ;[0.02137 0.1173 0.3385] Movimento Básico
  (bind _output_get (set `self.AxisX` AxisValue))
  (goto _label))

(event `Key|E`
  (params (Key :type "Key Structure"))
  (bind _returnvalue (`self.K2_GetActorLocation`))
  (bind _current_carriedmesh (`self.current_carriedMesh`))
  (bind _current_carriedmesh_2 (`self.current_carriedMesh`))
  (bind _grabbedactor (`self.GrabbedActor`))
  ;[0 0 0] Lógica de agarrar itens
  (:`Pressed`
    (if (`self.Iscarrying`)
      (`self.K2_DetachFromActor` (`self.GrabbedActor`) "KeepWorld" "KeepRelative" "KeepWorld")
      (set `self.Iscarrying` false)
      (`SceneComponent.SetVisibility` (`Actor.RootComponent` (`self.GrabbedActor`)) true true)
      (`NiagaraFunctionLibrary.SpawnSystemAtLocation` "/Game/VFX_Poof/P_Poof.P_Poof" (`SceneComponent.RelativeLocation` _current_carriedmesh) (`SceneComponent.RelativeRotation` _current_carriedmesh))
      (`PrimitiveComponent.SetSimulatePhysics` _current_carriedmesh true)
      (set `self.GrabbedActor` null)
      (`PrimitiveComponent.SetCollisionEnabled` _current_carriedmesh "QueryAndPhysics")
      (set `self.IsHolding` false)
      (else
        (bind (_outhit _returnvalue_2) (`KismetSystemLibrary.CapsuleTraceSingleForObjects` _returnvalue _returnvalue 120.0 100.0 (`|MakeArray` "ObjectTypeQuery4" :!type "EObjectTypeQuery Enum")))
        (if _returnvalue_2
          (bind (_bblockinghit _binitialoverlap _time _distance _location _impactpoint _normal _impactnormal _physmat _hitactor _hitcomponent) (`GameplayStatics.BreakHitResult` _outhit))
          (set `self.GrabbedActor` _hitactor)
          (set `self.current_carriedMesh` _hitcomponent)
          (set `self.Iscarrying` true)
          (`self.K2_AttachToComponent` (`self.GrabbedActor`) (`self.GrabPoint`) "None" "SnapToTarget" "SnapToTarget" "KeepWorld" true)
          (`SceneComponent.SetVisibility` (`Actor.RootComponent` _grabbedactor) false true)
          (set `self.Temp_Actor_Location` (`self.K2_GetActorLocation` _grabbedactor))
          (set `self.Temp_Actor_Rotator` (`self.K2_GetActorRotation` _grabbedactor))
          (`NiagaraFunctionLibrary.SpawnSystemAtLocation` "/Game/VFX_Poof/P_Poof.P_Poof" (`self.Temp_Actor_Location`) (`self.Temp_Actor_Rotator`) (5.0 5.0 5.0))
          (`PrimitiveComponent.SetSimulatePhysics` _current_carriedmesh_2 false)
          (`PrimitiveComponent.SetCollisionEnabled` _current_carriedmesh_2 "NoCollision")
          (set `self.IsHolding` true))))))

(fn `UserConstructionScript`)