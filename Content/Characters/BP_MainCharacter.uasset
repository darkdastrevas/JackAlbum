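; Player character Blueprint with world-axis movement, jumping and NPC dialogue interaction.
; Both input axes feed one normalized movement step that, while grounded, rotates the actor toward its velocity.
; Timed flags throttle jumping and briefly lock movement on landing.
; E calls TalkMessage through BPI_Dialog on overlapping NPCs, while a physics-constraint carry/drop routine is present but disconnected.
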(event `Key|E`
  (params (Key :type "Key Structure"))
  ;[1 1 1] salvo por preucaução
)

(event `self.OnLanded`
  (params (Hit :type "HitResult Structure (by ref)"))
  ;[0.09031 0.2878 0.6719] Logica do pulo
  (set `self.canMove` false)
  (`KismetSystemLibrary.Delay` 0.4)
  (set `self.isLanded` true)
  (set `self.canMove` true))

(event `InputAxis|Go Forwards/ Backwards`
  (params (AxisValue :type "Float (single-precision)"))
  (bind _returnvalue (`self.K2_GetActorLocation`))
  ;[0.02137 0.1173 0.3385] Movimento Básico
  (bind _output_get (set `self.AxisY` AxisValue))
  (if (`self.canMove`) :!label _label
    (bind _returnvalue_2 (`KismetMathLibrary.Normal` (`KismetMathLibrary.MakeVector` _output_get (stale `InputAxis|Go Right/ Left` _output_get))))
    (`self.AddMovementInput` _returnvalue_2)
    (if (and (not (`NavMovementComponent.IsFalling` (`self.CharacterMovement`))) (> (`KismetMathLibrary.VSize` _returnvalue_2) 0.1))
      (`self.K2_SetActorRotation` (`KismetMathLibrary.FindLookAtRotation` _returnvalue (+ _returnvalue (`self.GetVelocity`)))))))

(event `InputAction|Jump`
  (params (Key :type "Key Structure"))
  ;[0.09031 0.2878 0.6719] Logica do pulo
  (:`Pressed`
    (if (and (`self.isLanded`) (not (`self.IsJumping`)))
      (`self.Jump`)
      (set `self.IsJumping` true)
      (`KismetSystemLibrary.Delay` 0.75)
      (set `self.IsJumping` false))))

(event `InputAxis|Go Right/ Left`
  (params (AxisValue :type "Float (single-precision)"))
  ;[0.02137 0.1173 0.3385] Movimento Básico
  (bind _output_get (set `self.AxisX` AxisValue))
  (goto _label))

(event `Key|E`
  (params (Key :type "Key Structure"))
  (:`Pressed`
    (for _array_element (`self.GetOverlappingActors` "/Game/Dialogue/bp_npc.bp_npc_C")
      (if (`KismetSystemLibrary.DoesImplementInterface` _array_element "/Game/Dialogue/BPI_Dialog.BPI_Dialog_C")
        (message `/Game/Dialogue/BPI_Dialog.Talk` _array_element)))))

(fn `UserConstructionScript`)